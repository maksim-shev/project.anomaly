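; Trigger volume Blueprint that streams a level in and out and tracks whether the hero is inside a building.
; When the player pawn's root component enters TriggerBox, it sets IsInBuilding on HeroCharacter_BP and does a blocking load of LevelsToLoadNames, made visible.
; Any end overlap starts a non-blocking unload, without checking which component left, and clears the flag on the cached hero.
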(event OnComponentBeginOverlap(TriggerBox)
  (params (OverlappedComponent :type Primitive%20Component%20Object%20Reference) (OtherActor :type Actor%20Object%20Reference) (OtherComp :type Primitive%20Component%20Object%20Reference) (OtherBodyIndex :type Integer) (bFromSweep :type Boolean) (SweepResult :type Hit%20Result%20Structure%20%28by%20ref%29))
  (bind _returnvalue (Game|Player|GetPlayerPawn 0))
  (if (== OtherComp (Variables|/Script/Engine.Actor|GetRootComponent _returnvalue))
    (bind _ashero_character_bp (Utilities|Casting|CastToHeroCharacter_BP _returnvalue))
    (bind _output_get (Variables|Default|SetHeroCharacter _ashero_character_bp))
    (Variables|/Game/Characters/Hero/HeroCharacter_BP.HeroCharacter_BP_C|SetIsInBuilding _output_get true)
    (Game|LoadStreamLevel(byName) (Variables|Default|GetLevelsToLoadNames) true true)))

(event OnComponentEndOverlap(TriggerBox)
  (params (OverlappedComponent :type Primitive%20Component%20Object%20Reference) (OtherActor :type Actor%20Object%20Reference) (OtherComp :type Primitive%20Component%20Object%20Reference) (OtherBodyIndex :type Integer))
  (bind _herocharacter (Variables|Default|GetHeroCharacter))
  (Game|UnloadStreamLevel(byName) (Variables|Default|GetLevelsToLoadNames) false)
  (Utilities|IsValid _herocharacter
    (:Is%20Valid
      (Variables|/Game/Characters/Hero/HeroCharacter_BP.HeroCharacter_BP_C|SetIsInBuilding _herocharacter false))))

(fn ConstructionScript)