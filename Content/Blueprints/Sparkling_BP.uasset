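; Sparkling_BP is a hazard actor that repeatedly damages the hero character while it overlaps the actor.
; On begin overlap it casts to HeroCharacter_BP, stores the Hero and starts a looping timer with an interval derived from AttacksPerSecond.
; Each timer tick applies Damage to the stored Hero, and the timer is cleared by function name when that Hero ends the overlap.
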(event Custom|DamageTheHero
  (Game|Damage|ApplyDamage (Variables|Default|GetHero) (Variables|Default|GetDamage) 0 0))

(event Collision|EventActorEndOverlap
  (params (OtherActor :type Actor%20Object%20Reference))
  (if (== OtherActor (Variables|Default|GetHero))
    (Utilities|Time|ClearTimerbyFunctionName 0 "DamageTheHero")))

(event Collision|EventActorBeginOverlap
  (params (OtherActor :type Actor%20Object%20Reference))
  (bind _ashero_character_bp (Utilities|Casting|CastToHeroCharacter_BP OtherActor))
  (Variables|Default|SetHero _ashero_character_bp)
  (Utilities|Time|SetTimerbyEvent (delegate Custom|DamageTheHero) (/ 1.0 (Variables|Default|GetAttacksPerSecond)) true))

(fn ConstructionScript)