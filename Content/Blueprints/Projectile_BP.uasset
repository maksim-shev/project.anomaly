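; Projectile Blueprint for a laser shot that damages damageable actors it overlaps.
; On overlap with an actor implementing Damageable_I, it sends its Damage through AffectHealthMessage unless that actor carries the Friendly tag.
; Either way it plays a lasgun impact sound and laser spark particles, then destroys itself.
; Actors without the interface are ignored, so the projectile passes on through them.
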(event Collision|EventActorBeginOverlap
  (params (OtherActor :type Actor%20Object%20Reference))
  (bind _returnvalue (Transformation|GetActorTransform))
  (if (Utilities|DoesObjectImplementInterface OtherActor "/Game/Blueprints/Damageable_I.Damageable_I_C")
    (if (not (Actor|ActorHasTag OtherActor "Friendly"))
      (Class|DamageableI|AffectHealth(Message) OtherActor (Variables|Default|GetDamage)))
    (Audio|SpawnSoundAttached "/Game/Audio/234082__211redman112__lasgun-impact.234082__211redman112__lasgun-impact" (Variables|Default|GetProjectileCollision) "None" "0, 0, 0" "0, 0, 0" "KeepRelativeOffset" false 1.0 1.0 0.0 0 0)
    (Effects|SpawnEmitteratLocation "/Game/Particles/LaserSparks_P.LaserSparks_P" (.location _returnvalue) (.rotation _returnvalue))
    (Actor|DestroyActor)))

(fn ConstructionScript)