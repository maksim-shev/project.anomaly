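; Weapon Blueprint that fires projectiles in response to trigger pull and release events.
; A pull passes a DoOnce gate, fires immediately and sets a non-looping timer for one more shot, delayed by the inverse of RoundsPerSecond.
; Release clears the Fire timer by function name and resets the gate.
; Each shot plays a silenced laser sound on GunMesh and spawns Projectile_BP at ProjectileSpawnPoint.
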(event Custom|PullTrigger
  (Utilities|FlowControl|DoOnce false
    (:Completed
      (CallFunction|Fire)
      (Utilities|Time|SetTimerbyEvent (delegate Custom|Fire) (/ 1.0 (Variables|Default|GetRounds%20Per%20Second))))))

(event Custom|ReleaseTrigger
  (Utilities|Time|ClearTimerbyFunctionName 0 "Fire")
  (Utilities|FlowControl|DoOnce false) ; enters at Reset
)

(event Custom|Fire
  (Audio|SpawnSoundAttached "/Game/Audio/151022__bubaproducer__laser-shot-silenced.151022__bubaproducer__laser-shot-silenced" (Variables|Default|GetGunMesh) "None" "0, 0, 0" "0, 0, 0" "KeepRelativeOffset" false 1.0 1.0 0.0 0 0)
  (Game|SpawnActorfromClass "/Game/Blueprints/Projectile_BP.Projectile_BP_C" (Transformation|GetWorldTransform (Variables|Default|GetProjectileSpawnPoint)) "Undefined" 0 0))

(fn ConstructionScript)